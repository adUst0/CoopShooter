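; Super speed powerup Blueprint that temporarily doubles the walk speed of the player who activates it.
; On activation it stores that player, multiplies MaxWalkSpeed on their CharacterMovementComponent and prints a debug string.
; On expiry it halves that speed if the stored player is still valid, then calls the parent expiry handler.
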(event EventOnExpired
  (bind _activedforplayer (Variables|Default|GetActivedForPlayer))
  (bind _returnvalue (Actor|GetComponentbyClass _activedforplayer "/Script/Engine.CharacterMovementComponent"))
  (Utilities|IsValid _activedforplayer
    (:Is%20Valid
      (Variables|/Script/Engine.CharacterMovementComponent|SetMaxWalkSpeed _returnvalue (/ (Variables|/Script/Engine.CharacterMovementComponent|GetMaxWalkSpeed _returnvalue) 2.0)))
    (:Is%20Not%20Valid
      _))
  (|CallParentFunction))

(event EventOnActivated
  (params (ActiveFor :type Actor%20Object%20Reference))
  (bind _returnvalue (Actor|GetComponentbyClass ActiveFor "/Script/Engine.CharacterMovementComponent"))
  (Variables|Default|SetActivedForPlayer ActiveFor)
  (Variables|/Script/Engine.CharacterMovementComponent|SetMaxWalkSpeed _returnvalue (* (Variables|/Script/Engine.CharacterMovementComponent|GetMaxWalkSpeed _returnvalue) 2.0))
  (Development|PrintString "On Activated"))

(fn ConstructionScript)